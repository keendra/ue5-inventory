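; BP_Pickupable is a world pickup from an inventory system example that adds its item to the player's inventory when clicked.
; The construction script sets its child actor class from the item data's template actor.
; BeginPlay binds to the child actor's click event, and Collect adds the item to an inventory obtained through the example player state, destroying the pickup only if that succeeds.
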(event `self.ReceiveBeginPlay`
  (add `self.OnClicked` (`ChildActorComponent.ChildActor` (`self.ChildActor`)) (`|CreateDelegate` :!event `Collect`)))

(fn `Collect`
  (params (TouchedActor :type "Actor Object Reference") (ButtonPressed :type "Key Structure" :default "None"))
  (bind _itemdata (`self.ItemData`))
  (bind _playerstate (`/Game/InventorySystemExample/InventoryUtils.GetExamplePlayerState`))
  (bind _returnvalue (`InventoryFunctionLibrary.GetInventory` _playerstate _itemdata))
  (if (`Inventory.AddItem` _returnvalue _itemdata)
    (`self.K2_DestroyActor`)))

(fn `UserConstructionScript`
  (bind _itemdata (`self.ItemData`)
    (:`then`
      (bind _templateactor (`BaseItem.TemplateActor` _itemdata)
        (:`then`
          (`ChildActorComponent.SetChildActorClass` (`self.ChildActor`) _templateactor))
        (:`else`)))
    (:`else`)))